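; BP_Interactable is an item that changes colour while it has focus.
; On BeginPlay it creates a dynamic material instance on its Cube and caches the starting "Colour" parameter as the default.
; StartFocus and EndFocus call their parent implementations, then set that parameter to the focused colour or restore the cached default.
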(event EventBeginPlay
  ;[1 1 1] Storing Start Colour
  (bind _returnvalue (Rendering|Material|CreateDynamicMaterialInstance (Variables|Default|GetCube) 0 0 "None" :!class /Script/Engine.PrimitiveComponent))
  (bind _output_get (Variables|Default|SetMaterialInstance _returnvalue))
  (bind _returnvalue_2 (Rendering|Material|GetVectorParameterValue _output_get "Colour" :!class /Script/Engine.MaterialInstanceDynamic))
  (Variables|Default|SetDefaultColor _returnvalue_2))

(event EventStartFocus
  (|CallParentFunction)
  (Rendering|Material|SetVectorParameterValue (Variables|Default|GetMaterialInstance) "Colour" (Variables|Default|GetFocusedValue) :!class /Script/Engine.MaterialInstanceDynamic))

(event EventEndFocus
  (|CallParentFunction)
  (Rendering|Material|SetVectorParameterValue (Variables|Default|GetMaterialInstance) "Colour" (Variables|Default|GetDefaultColor) :!class /Script/Engine.MaterialInstanceDynamic))

(fn ConstructionScript)