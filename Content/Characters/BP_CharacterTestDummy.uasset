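; BP_CharacterTestDummy is a test dummy character Blueprint with mostly disconnected combat logic.
; Its only wired event clears IsAttacking when the PrimaryAttack input is released.
; Unreachable leftover chains cover damage through HealthComponent with floating text, toggling weapon draw and sheath montages, and attacking or drawing the weapon first.
; The construction script is empty.
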(event Input|ActionEvents|InputActionPrimaryAttack
  (params (Key :type Key%20Structure :default "None"))
  (:Released
    (Variables|Default|SetIsAttacking false)))

(event Input|ActionEvents|InputActionDrawSheatheWeapon
  (params (Key :type Key%20Structure :default "None")))

(fn ConstructionScript)