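; Player character Blueprint that owns the player's UI, weapon draw/sheathe montages and damage intake.
; BeginPlay creates the main UI, death screen and hidden passive skill tree, and binds the death delegate to show that screen.
; Input actions toggle inventory, character screen, skill tree and HUD, most also switching input mode and cursor.
; Damage reduces HealthComponent health through a test AnyDamage handler or the guarded ProcessIncomingDamage function.
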(event Custom|CharacterDeath
  (params (XPToAssign :type Integer))
  ;[0.5436 0.3684 1] UI Functions
  (CallFunction|DisplayDeathScreen))

(event EventBeginPlay
  (EventDispatchers|BindEventtoCharacterDeathDelegate (delegate Custom|CharacterDeath))
  (CallFunction|InitializePassiveSkillTree)
  ;[0.5436 0.3684 1] UI Functions
  (CallFunction|SetupUIWidgets))

(event Game|Damage|EventAnyDamage
  (params (Damage :type Float%20%28single-precision%29) (DamageType :type Damage%20Type%20Object%20Reference) (InstigatedBy :type Controller%20Object%20Reference) (DamageCauser :type Actor%20Object%20Reference))
  ;[1 1 1] TEST Element for UI
  (Class|HealthComponent|DecreaseCurrentHealth (Variables|Default|GetHealthComponent) Damage))

(event Input|ActionEvents|InputActionToggleStatusBars
  (params (Key :type Key%20Structure :default "None"))
  (bind _mainuiref (Variables|Default|GetMainUIRef))
  ;[0.5436 0.3684 1] UI Functions
  ;;[1 1 1] Toggle Main UI Visibility
  (:Pressed
    (Utilities|FlowControl|FlipFlop
      (:A
        (Widget|SetVisibility _mainuiref "Hidden"))
      (:B
        (Widget|SetVisibility _mainuiref "Visible")))))

(event Input|ActionEvents|InputActionCharacterAttributesScreen
  (params (Key :type Key%20Structure :default "None"))
  (bind _returnvalue (Game|GetPlayerController 0))
  (bind _mainuiref (Variables|Default|GetMainUIRef))
  (bind _wbp_characterscreen (Variables|/Game/UI_Elements/WBP_MainUI.WBP_MainUI_C|GetWBP_CharacterScreen _mainuiref))
  ;[0.5436 0.3684 1] UI Functions
  ;;[1 1 1] Toggle CharacterScreen
  (:Pressed
    (if (Variables|Default|GetCharacterScreenVisible)
      (Variables|Default|SetCharacterScreenVisible false)
      (Widget|SetVisibility _wbp_characterscreen "Hidden")
      (Input|SetInputModeGameOnly _returnvalue)
      (bind _output_get (Variables|/Script/Engine.PlayerController|SetbShowMouseCursor _returnvalue false))
      (bind _output_get_2 (Variables|/Script/Engine.PlayerController|SetbEnableMouseOverEvents _returnvalue _output_get))
      (Variables|/Script/Engine.PlayerController|SetbEnableClickEvents _returnvalue _output_get_2)
      (else
        (Variables|Default|SetCharacterScreenVisible true)
        (Widget|SetVisibility _wbp_characterscreen "Visible")
        (Input|SetInputModeGameandUI _returnvalue _wbp_characterscreen "DoNotLock" false)
        (bind _output_get_3 (Variables|/Script/Engine.PlayerController|SetbShowMouseCursor _returnvalue true))
        (bind _output_get_4 (Variables|/Script/Engine.PlayerController|SetbEnableMouseOverEvents _returnvalue _output_get_3))
        (Variables|/Script/Engine.PlayerController|SetbEnableClickEvents _returnvalue _output_get_4)))))

(event Input|ActionEvents|InputActionPassiveSkillTree
  (params (Key :type Key%20Structure :default "None"))
  (bind _returnvalue (Game|GetPlayerController 0))
  (bind _mainuiref (Variables|Default|GetMainUIRef))
  (bind _passiveskilltreewidgetref (Variables|Default|GetPassiveSkillTreeWidgetRef))
  ;[0.5436 0.3684 1] UI Functions
  ;;[1 1 1] Toggle Passive Skill Tree
  (:Pressed
    (Utilities|FlowControl|FlipFlop
      (:A
        (Widget|SetVisibility _passiveskilltreewidgetref "Visible")
        (Input|SetInputModeGameandUI _returnvalue _passiveskilltreewidgetref "DoNotLock" false)
        (Default|UpdateSkillTreeWidget _passiveskilltreewidgetref)
        (bind _output_get (Variables|/Script/Engine.PlayerController|SetbShowMouseCursor _returnvalue true))
        (bind _output_get_2 (Variables|/Script/Engine.PlayerController|SetbEnableMouseOverEvents _returnvalue _output_get))
        (Variables|/Script/Engine.PlayerController|SetbEnableClickEvents _returnvalue _output_get_2)
        (Widget|SetVisibility _mainuiref "Hidden"))
      (:B
        (Widget|SetVisibility _passiveskilltreewidgetref "Hidden")
        (Input|SetInputModeGameOnly _returnvalue)
        (bind _output_get_3 (Variables|/Script/Engine.PlayerController|SetbShowMouseCursor _returnvalue false))
        (bind _output_get_4 (Variables|/Script/Engine.PlayerController|SetbEnableMouseOverEvents _returnvalue _output_get_3))
        (Variables|/Script/Engine.PlayerController|SetbEnableClickEvents _returnvalue _output_get_4)
        (Widget|SetVisibility _mainuiref "Visible")))))

(event Input|ActionEvents|InputActionDrawSheatheWeapon
  (params (Key :type Key%20Structure :default "None"))
  (:Pressed
    (CallFunction|DrawSheathWeapon)))

(event Input|ActionEvents|InputActionInventory
  (params (Key :type Key%20Structure :default "None"))
  (bind _returnvalue (Game|GetPlayerController 0))
  (bind _mainuiref (Variables|Default|GetMainUIRef))
  (bind _wbp_inventory (Variables|/Game/UI_Elements/WBP_MainUI.WBP_MainUI_C|GetWBP_Inventory _mainuiref))
  ;[0.5436 0.3684 1] UI Functions
  ;;[1 1 1] Toggle Inventory
  (:Pressed
    (if (Widget|IsVisible _wbp_inventory)
      (Widget|SetVisibility _wbp_inventory "Hidden")
      (Input|SetInputModeGameOnly _returnvalue)
      (Variables|/Script/Engine.PlayerController|SetbShowMouseCursor _returnvalue false)
      (else
        (Widget|SetVisibility _wbp_inventory "Visible")
        (Input|SetInputModeGameandUI _returnvalue _wbp_inventory "DoNotLock" false)
        (Variables|/Script/Engine.PlayerController|SetbShowMouseCursor _returnvalue true)))))

(fn ConstructionScript)

(fn UISetupCrosshair
  (bind _returnvalue (UserInterface|CreateWidget "/Game/UI_Elements/MainUI_Elements/WBP_Crosshair.WBP_Crosshair_C"))
  (UserInterface|Viewport|AddtoViewport _returnvalue 0))

(fn UISetupSkilltree
  (bind _returnvalue (UserInterface|CreateWidget "/Game/UI_Elements/MainUI_Elements/WBP_PassiveSkilltree.WBP_PassiveSkilltree_C"))
  (UserInterface|Viewport|AddtoViewport _returnvalue 0)
  (bind _output_get (Variables|Default|SetPassiveSkillTreeWidgetRef _returnvalue))
  (Widget|SetVisibility _output_get "Hidden"))

(fn UISetupDeathScreen
  (bind _returnvalue (UserInterface|CreateWidget "/Game/UI_Elements/WPB_PlayerDeathNotif.WPB_PlayerDeathNotif_C"))
  (Variables|Default|SetPlayerDeathUI _returnvalue))

(fn UISetupMainUI
  (bind _returnvalue (UserInterface|CreateWidget "/Game/UI_Elements/WBP_MainUI.WBP_MainUI_C" (Game|GetPlayerController 0)))
  (bind _output_get (Variables|Default|SetMainUIRef _returnvalue))
  (UserInterface|Viewport|AddtoViewport _output_get 0))

(fn DisplayDeathScreen
  (bind _returnvalue (Game|GetPlayerController 0))
  (bind _playerdeathui (Variables|Default|GetPlayerDeathUI))
  ;[1 1 1] Character Death
  (if (not (Variables|Default|GetbCharacterDeathScreenDisplayed))
    (UserInterface|Viewport|AddtoViewport _playerdeathui 0)
    (Input|SetInputModeUIOnly _returnvalue _playerdeathui "DoNotLock")
    (bind _output_get (Variables|/Script/Engine.PlayerController|SetbShowMouseCursor _returnvalue true))
    (bind _output_get_2 (Variables|/Script/Engine.PlayerController|SetbEnableMouseOverEvents _returnvalue _output_get))
    (Variables|/Script/Engine.PlayerController|SetbEnableClickEvents _returnvalue _output_get_2)
    (Variables|Default|SetbCharacterDeathScreenDisplayed true)
    (Widget|SetVisibility (Variables|Default|GetMainUIRef) "Hidden")))

(fn SetupUIWidgets
  (CallFunction|UISetupDeathScreen)
  (CallFunction|UISetupMainUI))

(fn ProcessIncomingDamage
  (params (DamageValue :type Float%20%28single-precision%29))
  (bind _healthcomponent (Variables|Default|GetHealthComponent))
  (Utilities|IsValid _healthcomponent
    (:Is%20Valid
      (if (not (Variables|Default|GetbIsCharacterDead))
        (Class|HealthComponent|DecreaseCurrentHealth _healthcomponent DamageValue)))
    (:Is%20Not%20Valid
      (Development|PrintString "Error When reading Health Component" true true "(R=0.906250,G=0.000000,B=0.000000,A=1.000000)"))))

(fn DrawSheathWeapon
  (if (Variables|Default|GetHasWeaponDrawn)
    (Animation|PlayAnimMontage "/Game/Characters/Animation_Human/animations/WeaponSheath.WeaponSheath" 1.0 "None")
    (else
      (Animation|PlayAnimMontage "/Game/Characters/Animation_Human/animations/WeaponDraw.WeaponDraw" 1.0 "None"))))

(fn InitializePassiveSkillTree
  (bind _returnvalue (UserInterface|CreateWidget "/Game/UI_Elements/MainUI_Elements/WBP_PassiveSkilltree.WBP_PassiveSkilltree_C" (Game|GetPlayerController 0)))
  (UserInterface|Viewport|AddtoViewport _returnvalue 0)
  (bind _output_get (Variables|Default|SetPassiveSkillTreeWidgetRef _returnvalue))
  (Widget|SetVisibility _output_get "Hidden")
  (Default|UpdateSkillTreeWidget (Variables|Default|GetPassiveSkillTreeWidgetRef))
  (return))