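; Anim notify state for human attack animations that detects melee weapon hits on characters.
; Each tick it sphere-traces on the Camera channel between the WeaponDrawn and OnehandWeaponTip sockets, adding the hit actor to the attacker's AttackedActors.
; It calls OnActiveAbilityTriggered for each BaseCharacter listed, then removes it immediately, so one target can trigger again on later ticks.
; An unconnected branch holds direct OnAttacked and damage calls for NPCs and players.
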(fn ReceivedNotifyTick
  (params (MeshComp :type Skeletal%20Mesh%20Component%20Object%20Reference) (Animation :type Anim%20Sequence%20Base%20Object%20Reference) (FrameDeltaTime :type Float%20%28single-precision%29))
  (bind _returnvalue (Components|GetOwner MeshComp))
  (bind _output_get (LocalVariables|SetAttacker _returnvalue))
  (bind _asbase_character (Utilities|Casting|CastToBaseCharacter _output_get))
  (bind _output_get_2 (LocalVariables|SetAttackingBaseCharacter _asbase_character))
  (bind _outhit (Collision|SphereTraceByChannel MeshComp (Transformation|GetSocketLocation MeshComp "WeaponDrawn") (Transformation|GetSocketLocation MeshComp "OnehandWeaponTip") 25.0 "TraceTypeQuery2" false (Utilities|Array|MakeArray _returnvalue) "ForDuration"))
  (Utilities|Array|AddUnique (Variables|/Script/TharsilProto.BaseCharacter|GetAttackedActors _output_get_2) (.hitactor _outhit))
  (for _array_element (Variables|/Script/TharsilProto.BaseCharacter|GetAttackedActors _output_get_2)
    (bind _asbase_character_2 (Utilities|Casting|CastToBaseCharacter _array_element))
    (Class|BaseCharacter|OnActiveAbilityTriggered (LocalVariables|GetAttackingBaseCharacter) _asbase_character_2)
    (Utilities|Array|RemoveItem (Variables|/Script/TharsilProto.BaseCharacter|GetAttackedActors _output_get_2) _array_element))
  (return false))