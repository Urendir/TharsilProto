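; BP_CharacterPlayable is a playable character Blueprint that handles input for drawing, sheathing and attacking with a weapon.
; PrimaryAttack sets IsAttacking while held if the weapon is drawn, otherwise the press plays the draw montage and marks it drawn.
; DrawSheatheWeapon toggles HasWeaponDrawn, playing the matching draw or sheathe montage.
; The flags change immediately on input, without waiting for montages to finish, and no attack logic runs in this graph.
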(event Input|ActionEvents|InputActionPrimaryAttack
  (params (Key :type Key%20Structure :default "None"))
  (:Pressed
    (if (Variables|Default|GetHasWeaponDrawn)
      (Variables|Default|SetIsAttacking true)
      (else
        (Animation|PlayAnimMontage "/Game/Characters/Animation_Human/animations/WeaponDraw.WeaponDraw" 1.0 "None")
        (Variables|Default|SetHasWeaponDrawn true))))
  (:Released
    (Variables|Default|SetIsAttacking false)))

(event Input|ActionEvents|InputActionDrawSheatheWeapon
  (params (Key :type Key%20Structure :default "None"))
  (:Pressed
    (if (Variables|Default|GetHasWeaponDrawn)
      (Animation|PlayAnimMontage "/Game/Characters/Animation_Human/animations/WeaponSheath.WeaponSheath" 1.0 "None")
      (Variables|Default|SetHasWeaponDrawn false)
      (else
        (Animation|PlayAnimMontage "/Game/Characters/Animation_Human/animations/WeaponDraw.WeaponDraw" 1.0 "None")
        (Variables|Default|SetHasWeaponDrawn true)))))

(fn ConstructionScript)