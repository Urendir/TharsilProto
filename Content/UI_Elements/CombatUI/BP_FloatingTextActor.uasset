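; Actor that shows floating combat text in the world through a widget component and removes itself afterwards.
; Initialize stores the text, and BeginPlay passes it to the WBP_FloatyCombatText widget, so it must be set before BeginPlay runs.
; BeginPlay also binds to the widget's animation-finished event, with HandleAnimFinished destroying the actor when the animation ends.
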(event EventBeginPlay
  (bind _aswbp_floaty_combat_text (Utilities|Casting|CastToWBP_FloatyCombatText (UserInterface|GetUserWidgetObject (Variables|Default|GetWidget))))
  (EventDispatchers|BindEventtoOnAnimFinishedEvent _aswbp_floaty_combat_text (EventDispatchers|CreateEvent :!event HandleAnimFinished))
  (Default|Initialize _aswbp_floaty_combat_text (Variables|Default|GetText)))

(event EventInitialize
  (params (Text :type Text%20%28by%20ref%29))
  (Variables|Default|SetText Text))

(fn ConstructionScript)

(fn HandleAnimFinished
  ;[1 1 1] Destroy Actor when animation finished.
  (Actor|DestroyActor))